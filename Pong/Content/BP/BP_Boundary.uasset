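; BP_Boundary is a goal boundary for a Pong game that awards a point when a ball overlaps it.
; It caches the PongModeBase game mode on BeginPlay.
; On overlap it destroys the Ball, then uses the IsLeftGoal flag to increase either the player's or the AI's score through that game mode.
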(event `self.ReceiveBeginPlay`
  ;[1 1 1] Store Game Mode Ref
  (bind _aspong_mode_base (cast `PongModeBase` (`GameplayStatics.GetGameMode`)))
  (set `self.GameModeRef` _aspong_mode_base))

(event `self.ReceiveActorBeginOverlap`
  (params (OtherActor :type "Actor Object Reference"))
  (bind _gamemoderef (`self.GameModeRef`))
  ;[1 1 1] Score Logic
  (if true
    (bind _asball (cast `Ball` OtherActor))
    (`self.K2_DestroyActor` _asball)
    (if (`self.IsLeftGoal`)
      (`PongModeBase.IncreasePlayerScore` _gamemoderef)
      (else
        (`PongModeBase.IncreaseAIScore` _gamemoderef)))))

(fn `UserConstructionScript`)